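; BP_SubtractPoints is a red plate that takes one point from the player's score when touched.
; On BeginPlay it finds and caches the BP_ThirdPersonCharacter through GetActorOfClass.
; The StaticMesh begin-overlap event decrements that character's CurrentPlayerScore only while it is above zero.
; The overlap does not check which actor touched the plate, so any overlap costs the cached player a point.
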(event `self.ReceiveBeginPlay`
  (bind _returnvalue (`GameplayStatics.GetActorOfClass` "/Game/ThirdPerson/Blueprints/BP_ThirdPersonCharacter.BP_ThirdPersonCharacter_C"))
  (set `self.PlayerRef` _returnvalue))

(event `self.StaticMesh.OnComponentBeginOverlap`
  (params (OverlappedComponent :type "PrimitiveComponent Object Reference") (OtherActor :type "Actor Object Reference") (OtherComp :type "PrimitiveComponent Object Reference") (OtherBodyIndex :type Integer) (bFromSweep :type Boolean) (SweepResult :type "HitResult Structure (by ref)"))
  ;[1 1 1] If the current score of the player is greater than 0, decrease by 1 upon touching the red plate.
  (if (> (`/Game/ThirdPerson/Blueprints/BP_ThirdPersonCharacter.CurrentPlayerScore` (`self.PlayerRef`)) 0)
    (bind _result (`/Engine/EditorBlueprintResources/StandardMacros.DecrementInt` (`/Game/ThirdPerson/Blueprints/BP_ThirdPersonCharacter.CurrentPlayerScore` (`self.PlayerRef`)))
      (:`  `
        (set `/Game/ThirdPerson/Blueprints/BP_ThirdPersonCharacter.CurrentPlayerScore` _result (`self.PlayerRef`))))))

(fn `UserConstructionScript`)